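; BP_Gate is a gate that raises and lowers its static mesh on Open and Close events.
; Open plays the Gate timeline, which eases the mesh's relative Z between two fixed heights, and Close reverses it.
; For saving, GetSaveData stores the mesh's location in GateLocation and serializes the actor, and LoadfromSaveData unserializes it and restores that location.
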(event `Open`
  (bind _staticmesh (`self.StaticMesh`))
  (bind (_relativelocation_x _relativelocation_y) (`KismetMathLibrary.BreakVector` (`SceneComponent.RelativeLocation` _staticmesh)))
  (bind (_direction _alpha) (`Timeline|Gate` :!label _label)
    (:`Update`
      (`SceneComponent.K2_SetRelativeLocation` _staticmesh (`KismetMathLibrary.MakeVector` _relativelocation_x _relativelocation_y (`|EaseFunction` "EaseIn" _alpha 150.0 451.0)) false false))))

(event `Close`
  (goto _label :!via `Reverse`))

(event `self.LoadFromSaveData`
  (params (InRecord :type "SHActorSaveData Structure"))
  (`SHBlueprintFunctionLibrary.UnserializeActor` self InRecord)
  (`SceneComponent.K2_SetRelativeLocation` (`self.StaticMesh`) (`self.GateLocation`) false false))

(fn `GetSaveData`
  (returns (ReturnValue :type "SHActorSaveData Structure"))
  (set `self.GateLocation` (`SceneComponent.RelativeLocation` (`self.StaticMesh`)))
  (bind _returnvalue (`SHBlueprintFunctionLibrary.SerializeActor` self))
  (return _returnvalue))

(fn `UserConstructionScript`)