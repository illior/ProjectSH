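; Interactable keypad combination lock where the player enters a four-character code to match CorrectCode.
; Interaction starts cursor navigation over a 3x4 button grid, highlighted by material swaps, with prompts shown in the inventory widget.
; Apply reads the selected button's text label to append a character, clear with C or submit with E.
; Submission shows Accept or ERROR with sound, and a Tick timer then completes the lock or re-enables input after one second.
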(event `self.ReceiveTick`
  (params (DeltaSeconds :type "Float (single-precision)"))
  (if (not (`self.bAcceptInput`))
    (if (`self.bAcceptState`)
      (bind _output_get (set `self.Timer` (+ (`self.Timer`) DeltaSeconds)))
      (if (> _output_get 1.0)
        (`self.Reset`)
        (`self.Complete`)
        (`self.SetActorTickEnabled` false))
      (elif (`self.bErrorState`)
        (bind _output_get_2 (set `self.Timer` (+ (`self.Timer`) DeltaSeconds)))
        (if (> _output_get_2 1.0)
          (set `self.bAcceptInput` true)
          (set `self.bErrorState` false)
          (set `self.Timer` 0.0)
          (`self.Reset`))))))

(event `self.ReceiveBeginPlay`
  (`self.SetActorTickEnabled` false))

(event `Interacted`
  (params (ActivatedActor :type "SHInteractableActor Object Reference") (ActivatedBy :type "SHCharacter Object Reference"))
  (bind _output_get (set `self.ButtonPosition` (0.0 0.0)))
  (`PrimitiveComponent.SetMaterial` (`|GetArrayItem` (`self.Buttons`) (`self.PositionToIndex` _output_get)) 0 (`self.SelectMaterial`))
  (set `self.TextPosition` 0)
  (set `self.CurrentCode` (`|MakeArray` "" "" "" ""))
  (`self.SetActorTickEnabled` true)
  (`self.SetDescription`))

(event `self.SetDescription`
  (bind _returnvalue (`self.GetInventoryWidget`))
  (`parent.SetDescription`)
  (`SHInventoryWidget.SetApplyDescription` _returnvalue (`self.ApplyText`))
  (`SHInventoryWidget.SetCancelDescription` _returnvalue (`self.CancelText`))
  (`SHInventoryWidget.SetMoveDescription` _returnvalue (`self.MoveText`)))

(event `Reset`
  (set `self.TextPosition` 0)
  (set `self.CurrentCode` (`|MakeArray` "" "" "" ""))
  (`TextRenderComponent.K2_SetText` (`self.DisplayText`) "____"))

(event `self.ReceiveApply`
  (if (`self.bAcceptInput`)
    (`GameplayStatics.PlaySound2D` "/Game/Game/UI/Sounds/SW_Click.SW_Click" 1.0 1.0 0.0 null null)
    (bind _astext_render_component (cast `TextRenderComponent` (`SceneComponent.GetChildComponent` (`|GetArrayItem` (`self.Buttons`) (`self.PositionToIndex` (`self.ButtonPosition`))) 0)))
    (bind _returnvalue (`KismetTextLibrary.Conv_TextToString` (`TextRenderComponent.Text` _astext_render_component)))
    (switch `string` _returnvalue
      (:`Default`
        (if (< (`self.TextPosition`) 4)
          (`KismetArrayLibrary.Array_Set` (`self.CurrentCode`) (`self.TextPosition`) _returnvalue)
          (set `self.TextPosition` (+ (`self.TextPosition`) 1))
          (`self.UpdateText`)))
      (:`C`
        (`self.Reset`))
      (:`E`
        (`self.Insert`)))))

(event `Insert`
  (if (== (`KismetStringLibrary.JoinStringArray` (`self.CurrentCode`) "") (`self.CorrectCode`))
    (set `self.bAcceptInput` false)
    (set `self.bAcceptState` true)
    (`TextRenderComponent.K2_SetText` (`self.DisplayText`) "Accept")
    (`GameplayStatics.PlaySound2D` "/Engine/EditorSounds/Notifications/CompileSuccess_Cue.CompileSuccess_Cue" 1.0 1.0 0.0 null null)
    (`PrimitiveComponent.SetMaterial` (`self.Button12`) 0 (`self.DefaultMaterial`))
    (else
      (set `self.bAcceptInput` false)
      (set `self.bErrorState` true)
      (`TextRenderComponent.K2_SetText` (`self.DisplayText`) "ERROR")
      (`GameplayStatics.PlaySound2D` "/Engine/EditorSounds/Notifications/CompileFailed_Cue.CompileFailed_Cue" 1.0 1.0 0.0 null null))))

(event `self.ReceiveCancel`
  (if (`self.bAcceptInput`)
    (`PrimitiveComponent.SetMaterial` (`|GetArrayItem` (`self.Buttons`) (`self.PositionToIndex` (`self.ButtonPosition`))) 0 (`self.DefaultMaterial`))
    (`TextRenderComponent.K2_SetText` (`self.DisplayText`) "____")
    (`self.ResumeGame`)
    (`self.SetActorTickEnabled` false)))

(event `self.ReceiveMoveWithFrequency`
  (params (Value :type "Vector2D Structure"))
  (bind (_x _y) (`KismetMathLibrary.BreakVector2D` Value))
  (bind (_buttonposition_x _buttonposition_y) (`KismetMathLibrary.BreakVector2D` (`self.ButtonPosition`)))
  (if (`self.bAcceptInput`)
    (`PrimitiveComponent.SetMaterial` (`|GetArrayItem` (`self.Buttons`) (`self.PositionToIndex` (`self.ButtonPosition`))) 0 (`self.DefaultMaterial`))
    (bind _output_get (set `self.ButtonPosition` (`KismetMathLibrary.MakeVector2D` (`KismetMathLibrary.FClamp` (+ _x _buttonposition_x) 0.0 2.0) (`KismetMathLibrary.FClamp` (- _buttonposition_y _y) 0.0 3.0))))
    (`PrimitiveComponent.SetMaterial` (`|GetArrayItem` (`self.Buttons`) (`self.PositionToIndex` _output_get)) 0 (`self.SelectMaterial`))))

(fn `PositionToIndex`
  (params (Position :type "Vector2D Structure"))
  (returns (Index :type Integer))
  (bind (_x _y) (`KismetMathLibrary.BreakVector2D` Position))
  (return (`KismetMathLibrary.FTrunc` (+ _x (* _y 3.0)))))

(fn `UpdateText`
  (locals (OutputString :type String))
  (for _array_element (`self.CurrentCode`)
    (set `local.OutputString` (`KismetStringLibrary.Concat_StrStr` (`local.OutputString`) (`KismetMathLibrary.SelectString` "_" _array_element (`KismetStringLibrary.IsEmpty` _array_element)))))
  (`TextRenderComponent.K2_SetText` (`self.DisplayText`) (`KismetTextLibrary.Conv_StringToText` (`local.OutputString`))))

(fn `UserConstructionScript`
  (`KismetArrayLibrary.Array_Add` (`self.Buttons`) (`self.Button1`))
  (`KismetArrayLibrary.Array_Add` (`self.Buttons`) (`self.Button2`))
  (`KismetArrayLibrary.Array_Add` (`self.Buttons`) (`self.Button3`))
  (`KismetArrayLibrary.Array_Add` (`self.Buttons`) (`self.Button4`))
  (`KismetArrayLibrary.Array_Add` (`self.Buttons`) (`self.Button5`))
  (`KismetArrayLibrary.Array_Add` (`self.Buttons`) (`self.Button6`))
  (`KismetArrayLibrary.Array_Add` (`self.Buttons`) (`self.Button7`))
  (`KismetArrayLibrary.Array_Add` (`self.Buttons`) (`self.Button8`))
  (`KismetArrayLibrary.Array_Add` (`self.Buttons`) (`self.Button9`))
  (`KismetArrayLibrary.Array_Add` (`self.Buttons`) (`self.Button10`))
  (`KismetArrayLibrary.Array_Add` (`self.Buttons`) (`self.Button11`))
  (`KismetArrayLibrary.Array_Add` (`self.Buttons`) (`self.Button12`))
  (add `SHInteractableActor.OnInteracted` (`|CreateDelegate` :!event `Interacted`)))