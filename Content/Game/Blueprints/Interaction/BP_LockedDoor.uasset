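; A one-sided locked door that can only be unlocked when interacted with from the side its arrow component points toward.
; The construction script binds a handler to OnInteracted.
; The handler compares the direction from the interactor to the arrow against the arrow's forward vector, using a dot product angle test.
; It either clears IsDoorLocked or leaves the door locked, printing a message in both cases.
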(event `Interacted`
  (params (ActivatedActor :type "SHInteractableActor Object Reference") (ActivatedBy :type "SHCharacter Object Reference"))
  (bind _arrowcomponent (`self.ArrowComponent`))
  (if (< (`KismetMathLibrary.DegAcos` (`KismetMathLibrary.Dot_VectorVector` (`KismetMathLibrary.GetForwardVector` (`KismetMathLibrary.FindLookAtRotation` (`self.K2_GetActorLocation` ActivatedBy) (`SceneComponent.K2_GetComponentLocation` _arrowcomponent))) (`SceneComponent.GetForwardVector` _arrowcomponent))) 90.0)
    (`KismetSystemLibrary.PrintString` "Door close from the other side")
    (else
      (set `self.bIsDoorLocked` false)
      (`KismetSystemLibrary.PrintString` "You open it"))))

(fn `UserConstructionScript`
  (add `SHInteractableActor.OnInteracted` (`|CreateDelegate` :!event `Interacted`)))