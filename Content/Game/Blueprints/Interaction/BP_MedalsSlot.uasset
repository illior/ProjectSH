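; Interactive medal slot where the player inserts three medal quest items from the inventory to complete it.
; Using a matching item reveals its medal, consumes the item and lets Tick lower the medal to its target offset over about a second.
; Resuming the game waits while a medal moves, then the inventory reopens or the slot completes.
; Each medal's visibility and location persist through save data.
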(event `self.ReceiveBeginPlay`
  (`self.SetActorTickEnabled` false))

(event `self.ReceiveTick`
  (params (DeltaSeconds :type "Float (single-precision)"))
  (bind (_relativelocation_x _relativelocation_y _relativelocation_z) (`KismetMathLibrary.BreakVector` (`SceneComponent.RelativeLocation` (`self.ActiveMedal`))))
  (bind _returnvalue (- _relativelocation_z (* DeltaSeconds (- (`self.InitialOffset`) (`self.TargetOffset`)))))
  (if (`self.IsAnyMedalMove`)
    (if (< _returnvalue (`self.TargetOffset`))
      (`SceneComponent.K2_SetRelativeLocation` (`self.ActiveMedal`) (`KismetMathLibrary.MakeVector` _relativelocation_x _relativelocation_y (`self.TargetOffset`)) false false)
      (set `self.ActiveMedal` null)
      (if (== (`BlueprintMapLibrary.Map_Length` (`self.Items`)) 0)
        (`self.Complete`)
        (else
          (`self.ShowItems`)))
      (else
        (`SceneComponent.K2_SetRelativeLocation` (`self.ActiveMedal`) (`KismetMathLibrary.MakeVector` _relativelocation_x _relativelocation_y _returnvalue) false false)))))

(event `Interacted`
  (params (ActivatedActor :type "SHInteractableActor Object Reference") (ActivatedBy :type "SHCharacter Object Reference"))
  (`self.ShowItems`)
  (`self.SetActorTickEnabled` true))

(event `self.ReceiveCancel`
  (if (not (`self.IsAnyMedalMove`))
    (`self.ResumeGame`)))

(event `self.HideItems`
  (`parent.HideItems`)
  (if (not (`self.IsAnyMedalMove`))
    (`self.ResumeGame`)))

(event `self.SetDescription`
  (bind _returnvalue (`self.GetInventoryWidget`))
  (`parent.SetDescription`)
  (`SHInventoryWidget.SetMoveDescription` _returnvalue "")
  (`SHInventoryWidget.SetCancelDescription` _returnvalue "")
  (`SHInventoryWidget.SetApplyDescription` _returnvalue ""))

(event `self.LoadFromSaveData`
  (params (InRecord :type "SHActorSaveData Structure"))
  (`parent.LoadFromSaveData` InRecord)
  (`SceneComponent.SetVisibility` (`self.Medal1`) (`self.bVisibleMedal1`) true)
  (`SceneComponent.K2_SetRelativeLocation` (`self.Medal1`) (`self.LocationMedal1`) false false)
  (`SceneComponent.SetVisibility` (`self.Medal2`) (`self.bVisibleMedal2`) true)
  (`SceneComponent.K2_SetRelativeLocation` (`self.Medal2`) (`self.LocationMedal2`) false false)
  (`SceneComponent.SetVisibility` (`self.Medal3`) (`self.bVisibleMedal3`) true)
  (`SceneComponent.K2_SetRelativeLocation` (`self.Medal3`) (`self.LocationMedal3`) false false))

(fn `GetSaveData`
  (returns (ReturnValue :type "SHActorSaveData Structure"))
  (bind _medal1 (`self.Medal1`))
  (bind _medal2 (`self.Medal2`))
  (bind _medal3 (`self.Medal3`))
  (set `self.bVisibleMedal1` (`SceneComponent.bVisible` _medal1))
  (set `self.LocationMedal1` (`SceneComponent.RelativeLocation` _medal1))
  (set `self.bVisibleMedal2` (`SceneComponent.bVisible` _medal2))
  (set `self.LocationMedal2` (`SceneComponent.RelativeLocation` _medal2))
  (set `self.bVisibleMedal3` (`SceneComponent.bVisible` _medal3))
  (set `self.LocationMedal3` (`SceneComponent.RelativeLocation` _medal3))
  (bind _returnvalue (`parent.GetSaveData`))
  (return _returnvalue))

(fn `IsAnyMedalMove`
  (returns (Value :type Boolean))
  (return (`KismetSystemLibrary.IsValid` (`self.ActiveMedal`))))

(fn `ReceiveUseItem`
  (params (InItemData :type "SHItemData Object Reference"))
  (returns (ReturnValue :type Boolean))
  (locals (MeshComponent :type "StaticMeshComponent Object Reference"))
  (bind _asshquest_item (cast `SHQuestItem` (`SHItemData.Item` InItemData))
    (:`then`
      (bind (_value _returnvalue) (`BlueprintMapLibrary.Map_Find` (`self.Items`) _asshquest_item))
      (if _returnvalue
        (bind _output_get (set `self.ActiveMedal` _value))
        (`SceneComponent.SetVisibility` _output_get true true)
        (`self.HideItems`)
        (`BlueprintMapLibrary.Map_Remove` (`self.Items`) _asshquest_item)
        (`self.SetItemIsGarbage` (`local.InItemData`))
        (return true)
        (else
          (return false))))
    (:`CastFailed`
      (return false))))

(fn `UserConstructionScript`
  (add `SHInteractableActor.OnInteracted` (`|CreateDelegate` :!event `Interacted`))
  (`BlueprintMapLibrary.Map_Add` (`self.Items`) "/Game/Game/InventorySystem/Items/DA_Medal1.DA_Medal1" (`self.Medal1`))
  (`BlueprintMapLibrary.Map_Add` (`self.Items`) "/Game/Game/InventorySystem/Items/DA_Medal2.DA_Medal2" (`self.Medal2`))
  (`BlueprintMapLibrary.Map_Add` (`self.Items`) "/Game/Game/InventorySystem/Items/DA_Medal3.DA_Medal3" (`self.Medal3`)))