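; Interactable item slot that opens item selection on interaction and accepts only the test device, always returning false from ReceiveUseItem.
; Using the device moves its child actor along a spline via a Timeline that ticks while paused.
; It then briefly shows the text mapped to the item's gameplay tag, defaulting to and adding the Center tag if none matches, then hides both and resumes the game.
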(event `StartAnim`
  (bind _spline (`self.Spline`))
  (`self.HideItems`)
  (`self.SetActorHiddenInGame` (`ChildActorComponent.ChildActor` (`self.BP_II_TestDevice`)) false)
  (bind (_direction _alpha) (`Timeline|Timeline` :!via `PlayFromStart`)
    (:`Update`
      (`SceneComponent.K2_SetWorldLocationAndRotation` (`self.BP_II_TestDevice`) (`SplineComponent.GetLocationAtTime` _spline _alpha "World" false) (`SplineComponent.GetRotationAtTime` _spline _alpha "World" false) false false))
    (:`Finished`
      (set `self.bFindTag` false)
      (for _array_element (`BlueprintGameplayTagLibrary.BreakGameplayTagContainer` (`SHItemData.ItemTags` (`self.ItemData`)))
        (bind (_value _returnvalue) (`BlueprintMapLibrary.Map_Find` (`self.Values`) _array_element))
        (if _returnvalue
          (`TextRenderComponent.K2_SetText` (`self.TextRender`) _value)
          (set `self.bFindTag` true)
          (break)))
      (`SceneComponent.SetHiddenInGame` (`self.TextRender`) false false)
      (if (not (`self.bFindTag`))
        (`BlueprintGameplayTagLibrary.AddGameplayTag` (`SHItemData.ItemTags` (`self.ItemData`)) (struct :`TagName` "Item.TestItem.Center"))
        (`TextRenderComponent.K2_SetText` (`self.TextRender`) (`BlueprintMapLibrary.Map_Find` (`self.Values`) (struct :`TagName` "Item.TestItem.Center"))))
      (set `self.ItemData` null)
      (`KismetSystemLibrary.Delay` 1.0)
      (`self.SetActorHiddenInGame` (`ChildActorComponent.ChildActor` (`self.BP_II_TestDevice`)) true)
      (`SceneComponent.SetHiddenInGame` (`self.TextRender`) true false)
      (`self.ResumeGame`))))

(event `Interacted`
  (params (ActivatedActor :type "SHInteractableActor Object Reference") (ActivatedBy :type "SHCharacter Object Reference"))
  (`self.ShowItems`))

(event `self.HideItems`
  (`parent.HideItems`)
  (`/Engine/EditorBlueprintResources/StandardMacros.IsValid` (`self.ItemData`)
    (:`Is Not Valid`
      (`self.ResumeGame`)
      (`self.SetActorHiddenInGame` (`ChildActorComponent.ChildActor` (`self.BP_II_TestDevice`)) true))))

(fn `ReceiveUseItem`
  (params (InItemData :type "SHItemData Object Reference"))
  (returns (ReturnValue :type Boolean))
  (if (== (`SHItemData.Item` InItemData) "/Game/Game/InventorySystem/Items/DA_TestDevice.DA_TestDevice")
    (set `self.ItemData` (`local.InItemData`))
    (`self.StartAnim`)
    (return false)
    (else
      (return false))))

(fn `UserConstructionScript`
  (`self.SetActorEnableCollision` (`ChildActorComponent.ChildActor` (`self.BP_II_TestDevice`)) false)
  (add `SHInteractableActor.OnInteracted` (`|CreateDelegate` :!event `Interacted`))
  (`ActorComponent.SetTickableWhenPaused` (`self.Timeline`) true))