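; Test inventory interaction device with three buttons that set the gameplay tag on the current interact item target.
; Activating its Arrow point moves the target to its close-inspect location, then restores the button selection from its tags, defaulting to center.
; Menu move input shifts the overlay highlight, rewrites the tag and updates the TextRender.
; Cancel stops inspection and disables input; Apply prints the tags.
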(event `EnhancedInput|/Game/Game/Player/Input/Pause/IA_MenuApply`
  (params (ActionValue :type Boolean) (ElapsedSeconds :type "Float (double-precision)") (TriggeredSeconds :type "Float (double-precision)") (InputAction :type "InputAction Object Reference" :default "/Game/Game/Player/Input/Pause/IA_MenuApply.IA_MenuApply"))
  (:`Started`
    (for _array_element (`BlueprintGameplayTagLibrary.BreakGameplayTagContainer` (`SHItemData.ItemTags` (`SHInteractItemTarget.InteractItemData` (`self.GetInteractItemTarget`))))
      (`KismetSystemLibrary.PrintString` (`KismetStringLibrary.Conv_NameToString` (`BlueprintGameplayTagLibrary.GetTagName` _array_element))))))

(event `self.ActivateInteractPoint`
  (params (TargetComponent :type "SceneComponent Object Reference"))
  (bind _returnvalue (`self.GetInteractItemTarget`))
  (bind _interactitemdata (`SHInteractItemTarget.InteractItemData` (`self.GetInteractItemTarget`)))
  (if (== TargetComponent (`self.Arrow`))
    (`SHMoveItemAsyncAction.MoveItemToTarget` _returnvalue (`SceneComponent.K2_GetComponentToWorld` (`SHInteractItemTarget.CloseInspectLocation` _returnvalue)) 0.5
      (:`OnCompleted`
        (`SHInteractItemTarget.ActivateInput` _returnvalue)
        (if (`BlueprintGameplayTagLibrary.HasTag` (`SHItemData.ItemTags` _interactitemdata) (struct :`TagName` "Item.TestItem"))
          (for (_array_element _array_index) (`self.ButtonTags`)
            (if (`BlueprintGameplayTagLibrary.HasTag` (`SHItemData.ItemTags` (`SHInteractItemTarget.InteractItemData` (`self.GetInteractItemTarget`))) _array_element)
              (bind _output_get (set `self.Index` _array_index))
              (`MeshComponent.SetOverlayMaterial` (`|GetArrayItem` (`self. Buttons`) _output_get) (`self.OverlayMaterial`))
              (break)))
          (else
            (set `SHItemData.ItemTags` (struct :`GameplayTags` (struct :`(TagName` "Item.TestItem.Center"))) _interactitemdata)
            (bind _output_get_2 (set `self.Index` 1))
            (`MeshComponent.SetOverlayMaterial` (`|GetArrayItem` (`self. Buttons`) _output_get_2) (`self.OverlayMaterial`))))
        (`self.UpdateText`)))))

(event `EnhancedInput|/Game/Game/Player/Input/Pause/IA_MenuCancel`
  (params (ActionValue :type Boolean) (ElapsedSeconds :type "Float (double-precision)") (TriggeredSeconds :type "Float (double-precision)") (InputAction :type "InputAction Object Reference" :default "/Game/Game/Player/Input/Pause/IA_MenuCancel.IA_MenuCancel"))
  (:`Completed`
    (`MeshComponent.SetOverlayMaterial` (`|GetArrayItem` (`self. Buttons`) (`self.Index`)) null)
    (`KismetSystemLibrary.DelayUntilNextTick`)
    (`self.StopInspectItem`)
    (`self.DisableInput` (`GameplayStatics.GetPlayerController` 0))))

(event `EnhancedInput|/Game/Game/Player/Input/Pause/IA_MenuMove`
  (params (ActionValue :type "Vector2D Structure") (ElapsedSeconds :type "Float (double-precision)") (TriggeredSeconds :type "Float (double-precision)") (InputAction :type "InputAction Object Reference" :default "/Game/Game/Player/Input/Pause/IA_MenuMove.IA_MenuMove"))
  (bind _returnvalue (`KismetMathLibrary.Clamp` (+ (`self.Index`) (`KismetMathLibrary.BreakVector2D` ActionValue)) 0 (- (`KismetArrayLibrary.Array_Length` (`self. Buttons`)) 1)))
  (:`Started`
    (if (!= (`self.Index`) _returnvalue)
      (`MeshComponent.SetOverlayMaterial` (`|GetArrayItem` (`self. Buttons`) (`self.Index`)) null)
      (bind _output_get (set `self.Index` _returnvalue))
      (`MeshComponent.SetOverlayMaterial` (`|GetArrayItem` (`self. Buttons`) _output_get) (`self.OverlayMaterial`))
      (set `SHItemData.ItemTags` (`BlueprintGameplayTagLibrary.MakeGameplayTagContainerFromTag` (`|GetArrayItem` (`self.ButtonTags`) (`self.Index`))) (`SHInteractItemTarget.InteractItemData` (`self.GetInteractItemTarget`)))
      (`self.UpdateText`))))

(event `UpdateText`
  (switch `int` (`self.Index`)
    (:`0`
      (`TextRenderComponent.K2_SetText` (`self.TextRender`) "11 00 00"))
    (:`1`
      (`TextRenderComponent.K2_SetText` (`self.TextRender`) "00 11 00"))
    (:`2`
      (`TextRenderComponent.K2_SetText` (`self.TextRender`) "00 00 11"))))

(fn `GetInteractPoints`
  (returns (ReturnValue :type "Array of SceneComponent Object Reference"))
  (return (`|MakeArray` (`self.Arrow`) :!type "SceneComponent Object Reference")))

(fn `UserConstructionScript`
  (set `self. Buttons` (`|MakeArray` (`self.Button2`) (`self.Button1`) (`self.Button`))))